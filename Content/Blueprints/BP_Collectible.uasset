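; BP_Collectible is a spinning ammo pickup for the first-person character.
; Its mesh yaws by RotationSpeed each tick, without delta-time scaling.
; Overlapping PickupRadius casts the other actor's Instigator to BP_FirstPersonCharacter and adds a fixed amount to its Ammo.
; It then prints a debug total that re-adds the bonus, plays a sound at the world origin rather than the pickup, and destroys itself.
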(event `self.ReceiveTick`
  (params (DeltaSeconds :type "Float (single-precision)"))
  (`SceneComponent.K2_AddRelativeRotation` (`self.StaticMesh`) (`KismetMathLibrary.MakeRotator` 0.0 0.0 (`self.RotationSpeed`)) false false))

(event `self.PickupRadius.OnComponentBeginOverlap`
  (params (OverlappedComponent :type "PrimitiveComponent Object Reference") (OtherActor :type "Actor Object Reference") (OtherComp :type "PrimitiveComponent Object Reference") (OtherBodyIndex :type Integer) (bFromSweep :type Boolean) (SweepResult :type "HitResult Structure (by ref)"))
  (bind _asbp_first_person_character (cast `/Game/FirstPerson/Blueprints/BP_FirstPersonCharacter` (`self.GetInstigator` OtherActor)))
  (bind _returnvalue (+ 20 (`/Game/FirstPerson/Blueprints/BP_FirstPersonCharacter.Ammo` _asbp_first_person_character)))
  (set `/Game/FirstPerson/Blueprints/BP_FirstPersonCharacter.Ammo` _returnvalue _asbp_first_person_character)
  (`KismetSystemLibrary.PrintString` (`KismetStringLibrary.Conv_IntToString` _returnvalue))
  (`GameplayStatics.PlaySoundAtLocation` "/Game/SFX/box-of-ammo-64427.box-of-ammo-64427" (0.0 0.0 0.0) (struct) 1.0 1.0 0.0 null null null null)
  (`self.K2_DestroyActor`))

(fn `UserConstructionScript`)