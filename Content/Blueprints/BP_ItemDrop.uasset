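; BP_ItemDrop is a collectible pickup that spins in place and counts down the items remaining.
; Each tick yaws its static mesh by RotationSpeed, without scaling by delta time.
; Any overlap with PickupRadius, with no check on the other actor, decrements Remaining on BP_FirstPersonGameMode, adds a WB_Collected widget to the viewport and destroys the item.
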(event `self.PickupRadius.OnComponentBeginOverlap`
  (params (OverlappedComponent :type "PrimitiveComponent Object Reference") (OtherActor :type "Actor Object Reference") (OtherComp :type "PrimitiveComponent Object Reference") (OtherBodyIndex :type Integer) (bFromSweep :type Boolean) (SweepResult :type "HitResult Structure (by ref)"))
  (bind _asbp_first_person_game_mode (cast `/Game/FirstPerson/Blueprints/BP_FirstPersonGameMode` (`GameplayStatics.GetGameMode`)))
  (bind _result (`/Engine/EditorBlueprintResources/StandardMacros.DecrementInt` (`/Game/FirstPerson/Blueprints/BP_FirstPersonGameMode.Remaining` _asbp_first_person_game_mode))
    (:`  `
      (set `/Game/FirstPerson/Blueprints/BP_FirstPersonGameMode.Remaining` _result _asbp_first_person_game_mode)
      (bind _returnvalue (`|CreateWidget` "/Game/Blueprints/WB_Collected.WB_Collected_C"))
      (`UserWidget.AddToViewport` _returnvalue 0)
      (`self.K2_DestroyActor`))))

(event `self.ReceiveTick`
  (params (DeltaSeconds :type "Float (single-precision)"))
  (`SceneComponent.K2_AddRelativeRotation` (`self.StaticMesh`) (`KismetMathLibrary.MakeRotator` 0.0 0.0 (`self.RotationSpeed`)) false false))

(fn `UserConstructionScript`)