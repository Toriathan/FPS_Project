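; BP_Charging_Enemy is an enemy that runs at the player once spotted and destroys itself on attack.
; PawnSensing sets a seeing flag and starts AIMoveTo; on arrival it plays a montage, applies damage and destroys the actor.
; Overlapping a first-person projectile also destroys it.
; Tick halts movement until the flag is set, then repeatedly zeroes Health; the flag is never effectively cleared.
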(event `self.ReceiveTick`
  (params (DeltaSeconds :type "Float (single-precision)"))
  (`|ExecutionSequence`
    (:`then_0`
      (if (`self.isSeeingPlayer`)
        (set `self.Health` 0.0)
        (else
          (`MovementComponent.StopMovementImmediately` (`self.CharacterMovement`)))))))

(event `self.PawnSensing.OnSeePawn`
  (params (Pawn :type "Pawn Object Reference"))
  (set `self.isSeeingPlayer` true)
  (`self.FollowPlayer`))

(event `FollowPlayer`
  (set `self.canAttack` true)
  (if (`self.isSeeingPlayer`)
    (`|AIMoveTo` self (0.0 0.0 0.0) (`GameplayStatics.GetPlayerCharacter` 0) 70.0
      (:`OnSuccess`
        (if (`self.canAttack`)
          (set `self.canAttack` false)
          (`self.PlayAnimMontage` "/Game/Enemy/AI/AM_Enemy.AM_Enemy")
          (`GameplayStatics.ApplyDamage` (`GameplayStatics.GetPlayerCharacter` 0) 1.0)
          (`self.K2_DestroyActor`))))
    (else
      (set `self.isSeeingPlayer` false))))

(event `self.ReceiveActorBeginOverlap`
  (params (OtherActor :type "Actor Object Reference"))
  (cast `/Game/FirstPerson/Blueprints/BP_FirstPersonProjectile` OtherActor)
  (`self.K2_DestroyActor`))

(fn `UserConstructionScript`)