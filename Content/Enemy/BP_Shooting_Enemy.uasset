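; Shooting enemy that turns toward a seen player, attacks on a cooldown, and is destroyed when a first-person projectile overlaps it.
; PawnSensing sightings of BP_FirstPersonCharacter drive the rotation and the attack, which is gated by a CanAttack flag and Delay.
; Each attack spawns a projectile at SpawnProjectileLocation but damages the player immediately, independent of whether that projectile hits.
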(event `self.ReceiveActorBeginOverlap`
  (params (OtherActor :type "Actor Object Reference"))
  (cast `/Game/FirstPerson/Blueprints/BP_FirstPersonProjectile` OtherActor)
  (`self.K2_DestroyActor`))

(event `self.PawnSensing.OnSeePawn`
  (params (Pawn :type "Pawn Object Reference"))
  (bind _asbp_first_person_character (cast `/Game/FirstPerson/Blueprints/BP_FirstPersonCharacter` Pawn))
  (`self.K2_SetActorRotation` (`KismetMathLibrary.FindLookAtRotation` (`self.K2_GetActorLocation`) (`self.K2_GetActorLocation` _asbp_first_person_character)))
  (if (`self.CanAttack?`)
    (`|SpawnActorFromClass` "/Game/FirstPerson/Blueprints/BP_FirstPersonProjectile.BP_FirstPersonProjectile_C" (`SceneComponent.K2_GetComponentToWorld` (`self.SpawnProjectileLocation`)) "Undefined" "MultiplyWithRoot" null null)
    (`GameplayStatics.ApplyDamage` _asbp_first_person_character 10.0)
    (set `self.CanAttack?` false)
    (`KismetSystemLibrary.Delay` 1.5)
    (set `self.CanAttack?` true)))

(fn `UserConstructionScript`)